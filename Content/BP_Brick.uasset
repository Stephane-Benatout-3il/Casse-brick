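; BP_Brick is a brick actor that takes a random color when play begins.
; BeginPlay rolls one of five options, sets the matching yellow, blue, green, orange or red material instance on BrickMesh, and stores the corresponding color in BrickColor.
; The construction script is empty, so the color is chosen only at runtime, and no overlap or tick logic runs.
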(event `self.ReceiveBeginPlay`
  (bind _brickmesh (`self.BrickMesh`))
  (switch `int` (`KismetMathLibrary.RandomIntegerInRange` 0 4)
    (:`0`
      (`PrimitiveComponent.SetMaterial` _brickmesh 0 "/Game/Materials/MI_Brick_Yellow.MI_Brick_Yellow")
      (set `self.BrickColor` (struct :`R` 0.841 :`G` 0.785 :`B` 0.014 :`A` 1.0)))
    (:`1`
      (`PrimitiveComponent.SetMaterial` _brickmesh 0 "/Game/Materials/MI_Brick_Blue.MI_Brick_Blue")
      (set `self.BrickColor` (struct :`G` 0.552174 :`B` 1.0 :`A` 1.0)))
    (:`2`
      (`PrimitiveComponent.SetMaterial` _brickmesh 0 "/Game/Materials/MI_Brick_Green.MI_Brick_Green")
      (set `self.BrickColor` (struct :`G` 0.99 :`B` 0.013986 :`A` 1.0)))
    (:`3`
      (`PrimitiveComponent.SetMaterial` _brickmesh 0 "/Game/Materials/MI_Brick_Orange.MI_Brick_Orange")
      (set `self.BrickColor` (struct :`R` 1.0 :`G` 0.14522 :`A` 1.0)))
    (:`4`
      (`PrimitiveComponent.SetMaterial` _brickmesh 0 "/Game/Materials/MI_Brick_Red.MI_Brick_Red")
      (set `self.BrickColor` (struct :`R` 1.0 :`B` 0.014133 :`A` 1.0)))))

(fn `UserConstructionScript`)